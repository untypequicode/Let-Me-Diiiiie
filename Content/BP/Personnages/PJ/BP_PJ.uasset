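; Player character for a timed, level-based score game, handling movement, running and the menu, pause, tutorial and game-over HUDs.
; Emptying the Vie bar advances the level, adds a time-based score bonus, shrinks BP_Box, retunes damage, health and time, then teleports to PlayerStart behind a fade.
; A looping 0.1s timer triggers game over at zero.
; Scores, levels and records persist through SG_Score, with an intro shown when no save exists.
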(event Custom|SaveGame
  ;[1 1 1] SaveGame
  (bind _returnvalue (SaveGame|CreateSaveGameObject "/Game/BP/SG_Score.SG_Score_C"))
  (Utilities|Array|Add (Variables|/Game/BP/SG_Score.SG_Score_C|GetScores _returnvalue) (Variables|Score|GetScore))
  (Variables|/Game/BP/SG_Score.SG_Score_C|SetHighScore _returnvalue (Variables|Score|GetHighScore))
  (Utilities|Array|Add (Variables|/Game/BP/SG_Score.SG_Score_C|GetLevels _returnvalue) (Variables|Level|GetLevel))
  (Variables|/Game/BP/SG_Score.SG_Score_C|SetHighLevel _returnvalue (Variables|Level|GetHighLevel))
  (SaveGame|SaveGametoSlot _returnvalue "Score"))

(event Custom|AddScore/Level
  ;[1 1 1] AddScore
  (Utilities|Array|Add (Variables|Score|GetScores) (Variables|Score|GetScore))
  (Utilities|Array|Add (Variables|Level|GetLevels) (Variables|Level|GetLevel))
  (CallFunction|SearchHighScore/Level))

(event Custom|SearchHighScore/Level
  (bind _hud_menu (Variables|HUD|GetHUD_Menu))
  ;[1 1 1] SearchHighScore
  (Variables|Level|SetHighLvlTemp 0)
  (Variables|Score|SetHighScrTemp 0)
  (for _array_element (Variables|Score|GetScores)
    (if (> _array_element (Variables|Score|GetHighScrTemp))
      (Variables|Score|SetHighScrTemp _array_element)))
  (Variables|Score|SetHighScore (Variables|Score|GetHighScrTemp))
  (for _array_element_2 (Variables|Level|GetLevels)
    (if (> _array_element_2 (Variables|Level|GetHighLvlTemp))
      (Variables|Level|SetHighLvlTemp _array_element_2)))
  (Variables|Level|SetHighLevel (Variables|Level|GetHighLvlTemp))
  (CallFunction|SaveGame)
  (Utilities|IsValid _hud_menu
    (:Is%20Valid
      (Default|SetTextHighScore _hud_menu (Variables|Score|GetHighScore))
      (Default|SetTextHighLevel _hud_menu (Variables|Level|GetHighLevel)))))

(event Custom|Reset
  (params (Forward? :type Boolean))
  ;[1 1 1] Reset
  (Utilities|ResetPJ Forward?)
  (bind _outactors (Actor|GetAllActorsOfClass "/Game/BP/Personnages/IA/BP_Box.BP_Box_C"))
  (Transformation|SetWorldScale3D (Variables|/Game/BP/Personnages/IA/BP_Box.BP_Box_C|GetScene (Utilities|Array|Get(acopy) _outactors)) "1.000000,1.000000,1.000000")
  (Variables|Level|SetLevel 0)
  (Variables|Score|SetScore 0)
  (Variables|Time|SetTimeGame 6e+01)
  (Variables|Vie|SetVieMax 1e+02)
  (Variables|Vie|SetVie (Variables|Vie|GetVieMax))
  (Variables|Score|SetHighScrTemp 0)
  (Variables|Default|SetDegats 5.0)
  (Default|SetTextTimer (Variables|HUD|GetHUD_Main) (Variables|Time|GetTime))
  (Default|SetTextScore (Variables|HUD|GetHUD_Main) (Variables|Score|GetScore))
  (Default|SetTextLevel (Variables|HUD|GetHUD_Main) (Variables|Level|GetLevel))
  (Default|SetTextHighScore (Variables|HUD|GetHUD_Main) (Variables|Score|GetHighScore))
  (Default|SetTextHighLevel (Variables|HUD|GetHUD_Main) (Variables|Level|GetHighLevel)))

(event Custom|EventScore
  (params (AddScore :type Integer))
  ;[1 1 1] EventScore
  (Variables|Score|SetScore (+ (Variables|Score|GetScore) AddScore))
  (Utilities|IsValid (Variables|HUD|GetHUD_Main)
    (:Is%20Valid
      (Default|SetTextScore (Variables|HUD|GetHUD_Main) (Variables|Score|GetScore)))))

(event Custom|ChargeSaveGame
  (bind _hud_menu (Variables|HUD|GetHUD_Menu))
  ;[1 1 1] ChargeSaveGame
  (bind _returnvalue (SaveGame|DoesSaveGameExist "Score"))
  (if _returnvalue
    (bind _returnvalue_2 (SaveGame|LoadGamefromSlot "Score"))
    (bind _assg_score (Utilities|Casting|CastToSG_Score _returnvalue_2))
    (Utilities|Array|Clear (Variables|Score|GetScores))
    (Utilities|Array|Clear (Variables|Level|GetLevels))
    (Variables|Score|SetScores (Variables|/Game/BP/SG_Score.SG_Score_C|GetScores _assg_score))
    (Variables|Level|SetLevels (Variables|/Game/BP/SG_Score.SG_Score_C|GetLevels _assg_score))
    (bind _output_get (Variables|Score|SetHighScore (Variables|/Game/BP/SG_Score.SG_Score_C|GetHighScore _assg_score)))
    (bind _output_get_2 (Variables|Level|SetHighLevel (Variables|/Game/BP/SG_Score.SG_Score_C|GetHighLevel _assg_score)))
    (Utilities|IsValid _hud_menu
      (:Is%20Valid
        (Default|SetTextHighScore _hud_menu _output_get)
        (Default|SetTextHighLevel _hud_menu _output_get_2)))
    (else
      (Variables|Default|SetFirstGame true)
      (Utilities|IsValid (Variables|HUD|GetHUD_Intro)
        (:Is%20Valid
          _)
        (:Is%20Not%20Valid
          (bind _returnvalue_3 (UserInterface|CreateWidget "/Game/Widgets/HUD_Intro.HUD_Intro_C"))
          (Variables|HUD|SetHUD_Intro _returnvalue_3)))
      (UserInterface|Viewport|AddtoViewport (Variables|HUD|GetHUD_Intro) 0)
      (UserInterface|Animation|PlayAnimation (Variables|HUD|GetHUD_Intro) (Variables|/Game/Widgets/HUD_Intro.HUD_Intro_C|GetIntro (Variables|HUD|GetHUD_Intro)) 0.0 1 "Forward" 1.0 false))))

(event Custom|AddMenu
  (bind _returnvalue (Game|GetPlayerController 0))
  ;[1 1 1] HUD
  ;;[1 1 1] HUD Menu
  (if (not (Variables|Default|GetMenu?))
    (Variables|Default|SetMenu? true)
    (Utilities|IsValid (Variables|HUD|GetHUD_Menu)
      (:Is%20Not%20Valid
        (bind _returnvalue_2 (UserInterface|CreateWidget "/Game/Widgets/HUD_Menu.HUD_Menu_C"))
        (Variables|HUD|SetHUD_Menu _returnvalue_2)
        (if (UserInterface|Viewport|IsinViewport (Variables|HUD|GetHUD_Menu))
          _
          (else
            (UserInterface|Viewport|AddtoViewport _returnvalue_2 0)))
        (Variables|/Script/Engine.PlayerController|SetbShowMouseCursor _returnvalue true)
        (Input|SetInputModeGameandUI _returnvalue 0 "DoNotLock" true)
        (UserInterface|Animation|PlayAnimation _returnvalue_2 (Variables|/Game/Widgets/HUD_Menu.HUD_Menu_C|GetStart _returnvalue_2) 0.0 1 "Forward" 1.0 false)
        (Game|SetGamePaused true)))))

(event Custom|Add_HUDMain
  ;[1 1 1] HUD
  ;;[1 1 1] HUD Main
  (Utilities|IsValid (Variables|HUD|GetHUD_Main)
    (:Is%20Valid
      _)
    (:Is%20Not%20Valid
      (bind _returnvalue (UserInterface|CreateWidget "/Game/Widgets/HUD_Main.HUD_Main_C"))
      (Variables|HUD|SetHUD_Main _returnvalue)))
  (UserInterface|Viewport|AddtoViewport (Variables|HUD|GetHUD_Main) 0))

(event Custom|AddGame
  (bind _level (Variables|Level|GetLevel))
  (bind _returnvalue (Math|Conversions|ToFloat(Integer) _level))
  (bind _returnvalue_2 (/ _returnvalue 1e+02))
  (bind _returnvalue_3 (- 1.0 _returnvalue_2))
  ;[1 1 1] Addgame
  (Default|SetTextHighScore (Variables|HUD|GetHUD_Main) (Variables|Score|GetHighScore))
  (Default|SetTextHighLevel (Variables|HUD|GetHUD_Main) (Variables|Level|GetHighLevel))
  (CallFunction|EventScore (Math|Float|Truncate (/ (Variables|Time|GetTime) (/ 2.0 (Math|Conversions|ToFloat(Integer) (Variables|Level|GetLevel))))))
  (Default|SetTextLevel (Variables|HUD|GetHUD_Main) (Variables|Level|GetLevel))
  (bind _outactors (Actor|GetAllActorsOfClass "/Game/BP/Personnages/IA/BP_Box.BP_Box_C"))
  (Transformation|SetWorldScale3D (Variables|/Game/BP/Personnages/IA/BP_Box.BP_Box_C|GetScene (Utilities|Array|Get(acopy) _outactors)) (Math|Vector|MakeVector _returnvalue_3 _returnvalue_3 _returnvalue_3))
  (Variables|Default|SetDegats (/ (- 1.0 (/ (+ (Math|Conversions|ToFloat(Integer) (Variables|Level|GetLevel)) 2e+01) 5e+02)) 2.0))
  (Variables|Vie|SetVieMax (+ (* (Variables|Level|GetLevel) 5.0) (Variables|Vie|GetVieMax)))
  (Variables|Vie|SetVie (Variables|Vie|GetVieMax))
  (Variables|Time|SetTimeGame (- 3e+01 (* (Math|Conversions|ToFloat(Integer) (Variables|Level|GetLevel)) 0.5)))
  (Variables|Time|SetTime (Variables|Time|GetTimeGame))
  (Utilities|Time|SetTimerbyFunctionName 0 "Timer_" 0.1 true))

(event Custom|Start
  ;[1 1 1] Start
  (Variables|Default|SetStartAnim true)
  (Utilities|FlowControl|Delay 2.0)
  (Variables|Default|SetStartAnim false))

(event Custom|EventVie
  ;[1 1 1] EventVie
  (if (<= (- (Variables|Vie|GetVie) (Variables|Default|GetDegats)) 0.0)
    (bind _output_get (Variables|Vie|SetVie 0.0))
    (Default|SetProgVie (Variables|HUD|GetHUD_Main) _output_get)
    (Variables|Level|SetLevel (+ (Variables|Level|GetLevel) 1))
    (CallFunction|AddGame)
    (Utilities|IsValid (Variables|HUD|GetHUD_Victoire)
      (:Is%20Valid
        _)
      (:Is%20Not%20Valid
        (bind _returnvalue (UserInterface|CreateWidget "/Game/Widgets/HUD_Victoire.HUD_Victoire_C"))
        (Variables|HUD|SetHUD_Victoire _returnvalue)))
    (if (not (Widget|IsVisible (Variables|HUD|GetHUD_Victoire)))
      (UserInterface|Viewport|AddtoViewport (Variables|HUD|GetHUD_Victoire) 0)
      (Variables|Default|SetKeys? false)
      (Variables|Default|SetAxis%20Forward 0.0)
      (Variables|Default|SetAxis%20Right 0.0)
      (Variables|Default|SetDied? true)
      (Class|KismetSystemLibrary|PauseTimer 0 "Timer_")
      (UserInterface|Animation|PlayAnimation (Variables|HUD|GetHUD_Victoire) (Variables|/Game/Widgets/HUD_Victoire.HUD_Victoire_C|GetVictoire (Variables|HUD|GetHUD_Victoire)) 0.0 1 "Forward" 1.0 false)
      (Utilities|FlowControl|Delay 3.0)
      (Variables|Default|SetDied? false)
      (Widget|RemovefromParent (Variables|HUD|GetHUD_Victoire))
      (Utilities|ResetPJ true)
      (Class|KismetSystemLibrary|UnPauseTimer 0 "Timer_")
      (Variables|Default|SetKeys? true))
    (else
      (bind _output_get_2 (Variables|Vie|SetVie (- (Variables|Vie|GetVie) (Variables|Default|GetDegats))))
      (Default|SetProgVie (Variables|HUD|GetHUD_Main) _output_get_2))))

(event Custom|GameOver
  (bind _returnvalue (Game|GetPlayerController 0))
  ;[1 1 1] HUD
  ;;[1 1 1] HUD GameOver
  (CallFunction|AddScore/Level)
  (Utilities|IsValid (Variables|HUD|GetHUD_GameOver)
    (:Is%20Valid
      _)
    (:Is%20Not%20Valid
      (bind _returnvalue_2 (UserInterface|CreateWidget "/Game/Widgets/HUD_GameOver.HUD_GameOver_C"))
      (Variables|HUD|SetHUD_GameOver _returnvalue_2)))
  (UserInterface|Viewport|AddtoViewport (Variables|HUD|GetHUD_GameOver) 0)
  (Variables|/Script/Engine.PlayerController|SetbShowMouseCursor _returnvalue true)
  (Input|SetInputModeGameandUI _returnvalue 0 "DoNotLock" true)
  (UserInterface|Animation|PlayAnimation (Variables|HUD|GetHUD_GameOver) (Variables|/Game/Widgets/HUD_GameOver.HUD_GameOver_C|GetStart (Variables|HUD|GetHUD_GameOver)) 0.0 1 "Forward" 1.0 false))

(event EventBeginPlay
  (Audio|PlaySound2D "/Game/Sound/Fortuna.Fortuna" 1.0 1.0 0.0 0 0))

(event Collision|EventActorBeginOverlap
  (params (OtherActor :type Actor%20Object%20Reference)))

(event EventTick
  (params (DeltaSeconds :type Float%20%28single-precision%29)))

(event Input|ActionEvents|InputActionPause
  (params (Key :type Key%20Structure :default "None"))
  (bind _returnvalue (Game|GetPlayerController 0))
  (bind _hud_menu (Variables|HUD|GetHUD_Menu))
  (bind _hud_gameover (Variables|HUD|GetHUD_GameOver))
  ;[1 1 1] HUD
  ;;[1 1 1] HUD Pause
  (:Pressed
    (if (not (Game|IsGamePaused))
      (Utilities|IsValid _hud_menu
        (:Is%20Valid
          (if (not (Widget|IsVisible _hud_menu))
            (Utilities|IsValid _hud_gameover :!label _label
              (:Is%20Valid
                (if (not (Widget|IsVisible _hud_gameover))
                  (Game|SetGamePaused true :!label _label_2)
                  (Utilities|IsValid (Variables|HUD|GetHUD_Pause)
                    (:Is%20Valid
                      _)
                    (:Is%20Not%20Valid
                      (bind _returnvalue_2 (UserInterface|CreateWidget "/Game/Widgets/HUD_Pause.HUD_Pause_C"))
                      (Variables|HUD|SetHUD_Pause _returnvalue_2)))
                  (UserInterface|Viewport|AddtoViewport (Variables|HUD|GetHUD_Pause) 0)
                  (UserInterface|Animation|PlayAnimation (Variables|HUD|GetHUD_Pause) (Variables|/Game/Widgets/HUD_Pause.HUD_Pause_C|GetEnd (Variables|HUD|GetHUD_Pause)) 0.0 1 "Forward" 1.0 false)
                  (Variables|/Script/Engine.PlayerController|SetbShowMouseCursor _returnvalue true)
                  (Input|SetInputModeGameandUI _returnvalue 0 "DoNotLock" true)))
              (:Is%20Not%20Valid
                (goto _label_2)))))
        (:Is%20Not%20Valid
          (goto _label))))))

(event Input|ActionEvents|InputActionRun
  (params (Key :type Key%20Structure :default "None"))
  (bind _charactermovement (Variables|Character|GetCharacterMovement))
  ;[1 1 1] Running
  (:Pressed
    (Variables|Default|SetRun? true)
    (Variables|/Script/Engine.CharacterMovementComponent|SetMaxWalkSpeed _charactermovement 6e+02))
  (:Released
    (Variables|Default|SetRun? false)
    (Variables|/Script/Engine.CharacterMovementComponent|SetMaxWalkSpeed _charactermovement 3e+02)))

(event Input|AxisEvents|InputAxisMoveForward
  (params (AxisValue :type Float%20%28single-precision%29))
  ;[1 1 1] Move
  (if (Variables|Default|GetKeys?)
    (bind _output_get (Variables|Default|SetAxis%20Forward AxisValue))
    (Pawn|Input|AddMovementInput (Math|Vector|GetForwardVector (Math|Rotator|MakeRotator 0.0 0.0 (.yaw (Pawn|GetControlRotation :!class /Script/Engine.Pawn)))) (select (< (Variables|Default|GetAxis%20Forward) -0.75) -0.5 _output_get) false)))

(event Input|AxisEvents|InputAxisMoveRight
  (params (AxisValue :type Float%20%28single-precision%29))
  ;[1 1 1] Move
  (if (Variables|Default|GetKeys?)
    (Variables|Default|SetAxis%20Right AxisValue)
    (Pawn|Input|AddMovementInput (Math|Vector|GetRightVector (Math|Rotator|MakeRotator 0.0 0.0 (.yaw (Pawn|GetControlRotation :!class /Script/Engine.Pawn)))) AxisValue false)))

(fn ConstructionScript)

(fn AddHightScore
  (LocalVariables|SetHighScoreTemp 0)
  (for _array_element (Variables|Score|GetScores)
    (if (> _array_element (LocalVariables|GetHighScoreTemp))
      (LocalVariables|SetHighScoreTemp _array_element)))
  (Variables|Score|SetHighScore (LocalVariables|GetHighScoreTemp)))

(fn Timer
  (if (<= (- (Variables|Time|GetTime) 0.1) 0.0)
    (bind _output_get (Variables|Time|SetTime 0.0))
    (Default|SetTextTimer (Variables|HUD|GetHUD_Main) _output_get)
    (if (not (Game|IsGamePaused))
      (Game|SetGamePaused true)
      (CallFunction|GameOver)
      (CallFunction|AddScore/Level)
      (Default|SetTexts (Variables|HUD|GetHUD_GameOver) (Variables|Score|GetScore) (Variables|Score|GetHighScore) (Variables|Level|GetLevel) (Variables|Level|GetHighLevel))
      (Utilities|Time|ClearTimerbyFunctionName 0 "Timer_"))
    (else
      (bind _output_get_2 (Variables|Time|SetTime (- (Variables|Time|GetTime) 0.1)))
      (Default|SetTextTimer (Variables|HUD|GetHUD_Main) _output_get_2))))

(fn Tuto
  (bind _returnvalue (Game|GetPlayerController 0))
  (Utilities|IsValid (Variables|HUD|GetHUD_Tuto)
    (:Is%20Valid
      _)
    (:Is%20Not%20Valid
      (bind _returnvalue_2 (UserInterface|CreateWidget "/Game/Widgets/HUD_Tuto.HUD_Tuto_C"))
      (Variables|HUD|SetHUD_Tuto _returnvalue_2)))
  (UserInterface|Viewport|AddtoViewport (Variables|HUD|GetHUD_Tuto) 0)
  (Variables|/Script/Engine.PlayerController|SetbShowMouseCursor _returnvalue true)
  (Input|SetInputModeGameandUI _returnvalue 0 "DoNotLock" true)
  (UserInterface|Animation|PlayAnimation (Variables|HUD|GetHUD_Tuto) (Variables|/Game/Widgets/HUD_Tuto.HUD_Tuto_C|GetTuto (Variables|HUD|GetHUD_Tuto)) 0.0 1 "Forward" 1.0 false)
  (Game|SetGamePaused true))