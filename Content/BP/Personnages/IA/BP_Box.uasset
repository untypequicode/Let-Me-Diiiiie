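; BP_Box is a trigger actor that repeatedly calls the player's EventVie (life event) while BP_PJ stays inside its capsule.
; Begin overlap stores the player reference and starts a fast looping timer on EventLife, which forwards to EventVie; end overlap clears that timer.
; The In flag is set before the player cast on entry but only cleared for BP_PJ on exit, and is not read here.
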(event OnComponentBeginOverlap(Capsule)
  (params (OverlappedComponent :type Primitive%20Component%20Object%20Reference) (OtherActor :type Actor%20Object%20Reference) (OtherComp :type Primitive%20Component%20Object%20Reference) (OtherBodyIndex :type Integer) (bFromSweep :type Boolean) (SweepResult :type Hit%20Result%20Structure%20%28by%20ref%29))
  (Variables|Default|SetIn? true)
  (bind _asbp_pj (Utilities|Casting|CastToBP_PJ OtherActor))
  (Variables|Default|SetBP_PJ _asbp_pj)
  (Utilities|Time|SetTimerbyFunctionName 0 "EventLife" 0.01 true))

(event OnComponentEndOverlap(Capsule)
  (params (OverlappedComponent :type Primitive%20Component%20Object%20Reference) (OtherActor :type Actor%20Object%20Reference) (OtherComp :type Primitive%20Component%20Object%20Reference) (OtherBodyIndex :type Integer))
  (Utilities|Casting|CastToBP_PJ OtherActor)
  (Variables|Default|SetIn? false)
  (Utilities|Time|ClearTimerbyFunctionName 0 "EventLife"))

(event EventBeginPlay)

(event Collision|EventActorBeginOverlap
  (params (OtherActor :type Actor%20Object%20Reference)))

(event EventTick
  (params (DeltaSeconds :type Float%20%28single-precision%29)))

(fn ConstructionScript)

(fn EventLife
  (Default|EventVie (Variables|Default|GetBP_PJ)))