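; BP_IA is an AI character Blueprint that periodically randomises its animation state and plays the MonstreClue sound at its location on spawn.
; BeginPlay starts a looping half-second timer that calls the Timer function to count down.
; When the countdown runs out, the function rerolls a delay of a few seconds and picks one of seven Animation enum values at random.
; The graph contains no movement or perception logic.
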(event EventBeginPlay
  (Utilities|Time|SetTimerbyFunctionName 0 "Timer" 0.5 true)
  (Audio|PlaySoundatLocation "/Game/Sound/MonstreClue.MonstreClue" (Transformation|GetActorLocation) "0, 0, 0" 1.0 1.0 0.0 0 0 0))

(event Collision|EventActorBeginOverlap
  (params (OtherActor :type Actor%20Object%20Reference)))

(event EventTick
  (params (DeltaSeconds :type Float%20%28single-precision%29)))

(fn ConstructionScript)

(fn Timer
  (if (<= (- (Variables|Default|GetTime) 0.5) 0.0)
    (bind _output_get (Variables|Default|SetTimerMax (Math|Random|RandomFloatinRange 2.0 5.0)))
    (Variables|Default|SetTime _output_get)
    (Variables|Default|SetAnimation (Utilities|Select :Index (Math|Random|RandomIntegerinRange 0 6) :Option%200 "NewEnumerator0" :Option%201 "NewEnumerator1" :Option%202 "NewEnumerator2" :Option%203 "NewEnumerator3" :Option%204 "NewEnumerator4" :Option%205 "NewEnumerator5" :Option%206 "NewEnumerator6"))
    (else
      (Variables|Default|SetTime (- (Variables|Default|GetTime) 0.5)))))